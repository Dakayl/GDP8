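; CarSpawn is a spawner actor that periodically creates Car actors at its own location, limited by tokens from MyGameMode.
; A two-second Delay on Tick throttles attempts, each spawning only if GetToken succeeds, even when colliding.
; Each new car receives the spawner's orientation and speed, plus one of two direction-specific flipbooks, while its spawn rotation stays zero.
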(event EventBeginPlay)

(event EventActorBeginOverlap
  (params (OtherActor :type Actor%20Object%20Reference)))

(event EventTick
  (params (DeltaSeconds :type Float%20%28single-precision%29))
  (Utilities|FlowControl|Delay 2.0)
  (bind _asmy_game_mode (Utilities|Casting|CastToMyGameMode (Game|GetGameMode)))
  (bind _canspawn (Default|GetToken _asmy_game_mode))
  (if _canspawn
    (bind _returnvalue (Game|SpawnActorfromClass "/Game/Blueprints/Car.Car_C" (Math|Transform|MakeTransform (Transformation|GetActorLocation) (Class|KismetMathLibrary|MakeRot 0.0 0.0 0.0)) true 0))
    (Default|SetDirection _returnvalue (Variables|Default|GetEOrientation))
    (Sprite|SetFlipbook _returnvalue (select (Utilities|Enum|Equal(Enum) (Variables|Default|GetEOrientation) "NewEnumerator0") "/Game/FlipBooks/Car/CarFlipBookFinal.CarFlipBookFinal" "/Game/FlipBooks/Car/CarFlipBookFinalRight.CarFlipBookFinalRight"))
    (Variables|/Game/Blueprints/Car.Car_C|Setspeed _returnvalue (Variables|Default|Getspeed))))

(fn ConstructionScript)