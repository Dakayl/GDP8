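; Player hero, a flipbook-animated 2D character that moves on the X/Z plane, carries grandmas and dies on overlapping a car.
; The action input searches a sphere for the closest grabbable Grandma and slows flight while carrying; pressing again teleports her to the world origin.
; Axis inputs choose walk, carry and idle flipbooks by direction, while a timed Special state overrides them for throw, death and rebirth.
; Death halts movement, then notifies MyGameMode.
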(event OnComponentBeginOverlap(CapsuleComponent)
  (params (OtherActor :type Actor%20Object%20Reference) (OtherComp :type Primitive%20Component%20Object%20Reference) (OtherBodyIndex :type Integer) (bFromSweep :type Boolean) (SweepResult :type Hit%20Result%20Structure%20%28by%20ref%29))
  (Utilities|Casting|CastToCar OtherActor)
  (Pawn|Components|CharacterMovement|SetMovementMode "MOVE_None" 0)
  (Variables|Default|Setspecial true)
  (Variables|Default|SetheroSpecial "NewEnumerator0")
  (Utilities|FlowControl|Delay 0.67)
  (Variables|Default|Setspecial false)
  (Variables|Default|SetheroSpecial "NewEnumerator1")
  (bind _asmy_game_mode (Utilities|Casting|CastToMyGameMode (Game|GetGameMode)))
  (Default|HeroDeath _asmy_game_mode))

(event Custom|Rebirth
  (Variables|Default|Setspecial true)
  (Variables|Default|SetheroSpecial "NewEnumerator2")
  (Utilities|FlowControl|Delay 0.67)
  (Variables|Default|Setspecial false)
  (Variables|Default|SetheroSpecial "NewEnumerator1"))

(event Input|ActionEvents|InputActionAction
  (:Pressed
    (if (Variables|Default|GetgrandmaGrabbed)
      (CallFunction|ReleaseGrandma)
      (Utilities|FlowControl|Delay 0.67)
      (Variables|Default|Setspecial false)
      (Pawn|Components|CharacterMovement|SetMovementMode "MOVE_Flying" 0)
      (else
        ;[1 1 1] réinitialisation
        (Variables|Default|SetgrandmaDetected false)
        (Variables|Default|SetcurrentDistance (+ (Variables|Default|Getgrab%20Range) 6e+01))
        (bind _outactors (Class|KismetSystemLibrary|SphereOverlapActorsNEW (Transformation|GetActorLocation) (Variables|Default|Getgrab%20Range) (Utilities|Array|MakeArray "ObjectTypeQuery2") "/Game/Blueprints/Grandma.Grandma_C"))
        (for _array_element _outactors
          (bind _asgrandma (Utilities|Casting|CastToGrandma _array_element))
          (bind _cangrab (Default|CanGrab _asgrandma))
          (if _cangrab
            (if (< (Transformation|GetDistanceTo _asgrandma self) (Variables|Default|GetcurrentDistance))
              (Variables|Default|SetcurrentDistance (Transformation|GetDistanceTo _asgrandma self))
              (bind _output_get (Variables|Default|SetcurrentGrandma _asgrandma))
              (Variables|Default|SetgrandmaDetected true)
              (Default|GrabGrandma _output_get))))
        (if (Variables|Default|GetgrandmaDetected)
          (CallFunction|GrabGrandma))))))

(event Input|AxisEvents|InputAxisHorizontal
  (params (AxisValue :type Float%20%28single-precision%29))
  (bind _sprite (Variables|Default|GetSprite))
  (bind _grandmagrabbed (Variables|Default|GetgrandmaGrabbed))
  (bind _sprite_2 (Variables|Default|GetSprite))
  (if (Variables|Default|Getspecial)
    (switch Utilities|FlowControl|Switch|SwitchonHeroSpecial (Variables|Default|GetheroSpecial)
      (:NewEnumerator0
        (Sprite|SetFlipbook))
      (:NewEnumerator1
        (switch Utilities|FlowControl|Switch|SwitchonGrandmaDirection (Variables|Default|Getdirection)
          (:NewEnumerator0
            (Sprite|SetFlipbook _sprite_2 "/Game/FlipBooks/Hero/Launch/h_lance_dos_f.h_lance_dos_f"))
          (:NewEnumerator1
            (Sprite|SetFlipbook _sprite_2 "/Game/FlipBooks/Hero/Launch/h_lance_face_f.h_lance_face_f"))
          (:NewEnumerator2
            (Sprite|SetFlipbook _sprite_2 "/Game/FlipBooks/Hero/Launch/h_lance_gauche_f.h_lance_gauche_f"))
          (:NewEnumerator3
            (Sprite|SetFlipbook _sprite_2 "/Game/FlipBooks/Hero/Launch/h_lance_droite_f.h_lance_droite_f"))))
      (:NewEnumerator2
        (Sprite|SetFlipbook)))
    (elif (!= AxisValue 0.0)
      (Pawn|Input|AddMovementInput "1.000000, 0, 0" AxisValue false)
      (if (== (stale Input|AxisEvents|InputAxisVertical AxisValue) 0.0)
        (if (> AxisValue 0.0)
          (if _grandmagrabbed
            (Sprite|SetFlipbook "/Game/FlipBooks/Hero/Carry/hero_carry_right.hero_carry_right")
            (else
              (Sprite|SetFlipbook _sprite "/Game/FlipBooks/Hero/hero_WalkRight.hero_WalkRight")))
          (Variables|Default|Setdirection "NewEnumerator3")
          (else
            (if _grandmagrabbed
              (Sprite|SetFlipbook "/Game/FlipBooks/Hero/Carry/hero_carry_left.hero_carry_left")
              (else
                (Sprite|SetFlipbook _sprite "/Game/FlipBooks/Hero/hero_WalkLeft.hero_WalkLeft")))
            (Variables|Default|Setdirection "NewEnumerator2"))))
      (elif (not (> (Math|Vector|VectorLength (Transformation|GetVelocity)) 0.0))
        (if (Variables|Default|GetgrandmaGrabbed)
          (switch Utilities|FlowControl|Switch|SwitchonGrandmaDirection (Variables|Default|Getdirection)
            (:NewEnumerator0
              (Sprite|SetFlipbook "/Game/FlipBooks/Hero/Idle/h_porte_dos_idle_f.h_porte_dos_idle_f"))
            (:NewEnumerator1
              (Sprite|SetFlipbook "/Game/FlipBooks/Hero/Idle/h_porte_face_idle_f.h_porte_face_idle_f"))
            (:NewEnumerator2
              (Sprite|SetFlipbook "/Game/FlipBooks/Hero/Idle/h_porte_gauche_idle_f.h_porte_gauche_idle_f"))
            (:NewEnumerator3
              (Sprite|SetFlipbook "/Game/FlipBooks/Hero/Idle/h_porte_droite_idle_f.h_porte_droite_idle_f")))
          (else
            (switch Utilities|FlowControl|Switch|SwitchonGrandmaDirection (Variables|Default|Getdirection)
              (:NewEnumerator0
                (Sprite|SetFlipbook "/Game/FlipBooks/Hero/Idle/h_idle_dos_f.h_idle_dos_f"))
              (:NewEnumerator1
                (Sprite|SetFlipbook "/Game/FlipBooks/Hero/Idle/h_idle_face_f.h_idle_face_f"))
              (:NewEnumerator2
                (Sprite|SetFlipbook "/Game/FlipBooks/Hero/Idle/h_idle_gauche_f.h_idle_gauche_f"))
              (:NewEnumerator3
                (Sprite|SetFlipbook "/Game/FlipBooks/Hero/Idle/h_idle_droite_f.h_idle_droite_f")))))))))

(event Input|AxisEvents|InputAxisVertical
  (params (AxisValue :type Float%20%28single-precision%29))
  (bind _grandmagrabbed (Variables|Default|GetgrandmaGrabbed))
  (if (Variables|Default|Getspecial)
    (switch Utilities|FlowControl|Switch|SwitchonHeroSpecial "NewEnumerator0"
      (:NewEnumerator0
        (Sprite|SetFlipbook))
      (:NewEnumerator1
        (switch Utilities|FlowControl|Switch|SwitchonGrandmaDirection (Variables|Default|Getdirection)
          (:NewEnumerator0
            (Sprite|SetFlipbook "/Game/FlipBooks/Hero/Launch/h_lance_dos_f.h_lance_dos_f"))
          (:NewEnumerator1
            (Sprite|SetFlipbook "/Game/FlipBooks/Hero/Launch/h_lance_face_f.h_lance_face_f"))
          (:NewEnumerator2
            (Sprite|SetFlipbook "/Game/FlipBooks/Hero/Launch/h_lance_gauche_f.h_lance_gauche_f"))
          (:NewEnumerator3
            (Sprite|SetFlipbook "/Game/FlipBooks/Hero/Launch/h_lance_droite_f.h_lance_droite_f"))))
      (:NewEnumerator2
        (Sprite|SetFlipbook)))
    (elif (!= AxisValue 0.0)
      (Pawn|Input|AddMovementInput "0.000000,0.000000,1.000000" AxisValue false)
      (if (> AxisValue 0.0)
        (if _grandmagrabbed
          (Sprite|SetFlipbook "/Game/FlipBooks/Hero/Carry/hero_carry_up.hero_carry_up")
          (else
            (Sprite|SetFlipbook "/Game/FlipBooks/Hero/hero_WalkUp.hero_WalkUp")))
        (Variables|Default|Setdirection "NewEnumerator0")
        (else
          (if _grandmagrabbed
            (Sprite|SetFlipbook "/Game/FlipBooks/Hero/Carry/hero_carry_down.hero_carry_down")
            (else
              (Sprite|SetFlipbook "/Game/FlipBooks/Hero/hero_WalkDown.hero_WalkDown")))
          (Variables|Default|Setdirection "NewEnumerator1")))
      (elif (not (> (Math|Vector|VectorLength (Transformation|GetVelocity)) 0.0))
        (if (Variables|Default|GetgrandmaGrabbed)
          (switch Utilities|FlowControl|Switch|SwitchonGrandmaDirection (Variables|Default|Getdirection)
            (:NewEnumerator0
              (Sprite|SetFlipbook "/Game/FlipBooks/Hero/Idle/h_porte_dos_idle_f.h_porte_dos_idle_f"))
            (:NewEnumerator1
              (Sprite|SetFlipbook "/Game/FlipBooks/Hero/Idle/h_porte_face_idle_f.h_porte_face_idle_f"))
            (:NewEnumerator2
              (Sprite|SetFlipbook "/Game/FlipBooks/Hero/Idle/h_porte_gauche_idle_f.h_porte_gauche_idle_f"))
            (:NewEnumerator3
              (Sprite|SetFlipbook "/Game/FlipBooks/Hero/Idle/h_porte_droite_idle_f.h_porte_droite_idle_f")))
          (else
            (switch Utilities|FlowControl|Switch|SwitchonGrandmaDirection (Variables|Default|Getdirection)
              (:NewEnumerator0
                (Sprite|SetFlipbook "/Game/FlipBooks/Hero/Idle/h_idle_dos_f.h_idle_dos_f"))
              (:NewEnumerator1
                (Sprite|SetFlipbook "/Game/FlipBooks/Hero/Idle/h_idle_face_f.h_idle_face_f"))
              (:NewEnumerator2
                (Sprite|SetFlipbook "/Game/FlipBooks/Hero/Idle/h_idle_gauche_f.h_idle_gauche_f"))
              (:NewEnumerator3
                (Sprite|SetFlipbook "/Game/FlipBooks/Hero/Idle/h_idle_droite_f.h_idle_droite_f")))))))))

(fn ConstructionScript)

(fn GrabGrandma
  (Variables|Default|SetgrandmaGrabbed true)
  (Development|PrintString "Grabbed!")
  (Variables|/Script/Engine.CharacterMovementComponent|SetMaxFlySpeed (Variables|Character|GetCharacterMovement) 1e+02))

(fn ReleaseGrandma
  (Variables|Default|SetgrandmaGrabbed false)
  (Variables|/Script/Engine.CharacterMovementComponent|SetMaxFlySpeed (Variables|Character|GetCharacterMovement) 4e+02)
  (Variables|Default|Setspecial true)
  (Pawn|Components|CharacterMovement|SetMovementMode "MOVE_None" 0)
  (Transformation|Teleport (Variables|Default|GetcurrentGrandma) "0, 0, 0" "0, 0, 0"))