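; Car is a moving hazard actor that kills Grandma actors it overlaps.
; Each tick it counts down a lifetime and destroys itself at zero, otherwise sliding along its relative X axis at Speed, signed by Direction, which SetDirection assigns.
; Kills come from polling overlapping Grandmas every tick, limited to those at a similar height; an equivalent begin-overlap version is left disconnected.
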(event EventBeginPlay)

(event EventTick
  (params (DeltaSeconds :type Float%20%28single-precision%29))
  (Variables|Default|SetdestructIn (- (Variables|Default|GetdestructIn) DeltaSeconds))
  (if (<= (Variables|Default|GetdestructIn) 0.0)
    (Actor|DestroyActor)
    (else
      (for _array_element (Collision|GetOverlappingActors "/Game/Blueprints/Grandma.Grandma_C" :!class /Script/Engine.PrimitiveComponent)
        (bind _asgrandma (Utilities|Casting|CastToGrandma _array_element))
        (if (< (Math|Float|Absolute(Float) (- (.Z (Math|Vector|BreakVector (Transformation|GetActorLocation _asgrandma))) (.Z (Math|Vector|BreakVector (Transformation|GetActorLocation))))) 9e+01)
          (Default|Kill _asgrandma)))
      (Transformation|AddRelativeLocation (Math|Vector|MakeVector (* DeltaSeconds (select (Utilities|Enum|Equal(Enum) (Variables|Default|Getdirection) "NewEnumerator0") -1.0 1.0) (Variables|Default|Getspeed)) 0.0 0.0) false))))

(event EventActorBeginOverlap
  (params (OtherActor :type Actor%20Object%20Reference)))

(fn ConstructionScript)

(fn SetDirection
  (params (incomingDirection :type CarDirection%20Enum :default "NewEnumerator0"))
  (Variables|Default|Setdirection incomingDirection))