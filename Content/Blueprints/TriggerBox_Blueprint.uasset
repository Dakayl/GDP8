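; Trigger box Blueprint that serves as an arrival zone for Grandma actors.
; On overlap, it checks that the actor is a Grandma, that this box is her assigned ArrivalZone and that the player is not carrying her.
; When all checks pass, it switches her AiState to another enum state.
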(event EventBeginPlay)

(event EventTick
  (params (DeltaSeconds :type Float%20%28single-precision%29)))

(event EventActorBeginOverlap
  (params (OtherActor :type Actor%20Object%20Reference))
  (if (== (Utilities|GetClass OtherActor) "/Game/Blueprints/Grandma.Grandma_C")
    (bind _asgrandma (Utilities|Casting|CastToGrandma OtherActor))
    (if (== (Variables|/Game/Blueprints/Grandma.Grandma_C|GetarrivalZone _asgrandma) self)
      (if (not (Variables|/Game/Blueprints/Grandma.Grandma_C|GetisCarriedByPlayer _asgrandma))
        (Variables|/Game/Blueprints/Grandma.Grandma_C|SetAiState _asgrandma "NewEnumerator3")))))

(fn ConstructionScript)