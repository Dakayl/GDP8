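; Grandma actor: a pedestrian NPC that walks to a crosswalk, crosses the road, and can be carried by the player.
; Tick runs an AiState machine that walks, waits on a countdown, crosses toward FinalDestination, then destroys the actor after a delay.
; GrabGrandma forces Crossing and pauses her movement unless she has arrived; DropGrandma resumes it.
; Movement uses fixed per-frame relative offsets, and arrival is checked only while not carried.
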(event EventBeginPlay)

(event EventActorBeginOverlap
  (params (OtherActor :type Actor%20Object%20Reference)))

(event EventTick
  (params (DeltaSeconds :type Float%20%28single-precision%29))
  (switch Utilities|FlowControl|Switch|SwitchonGrandmaAIState (Variables|Default|GetAiState)
    (:NewEnumerator2
      ;[1 1 1] Walk towards crosswalk
      (Transformation|AddRelativeLocation "0.000000,-3.000000, 0" false)
      (if (Math|Vector|Equal(Vector) (Transformation|GetActorLocation) (Variables|Default|GetcrosswalkPosition) 5.0)
        (Variables|Default|SetAiState "NewEnumerator1")))
    (:NewEnumerator1
      ;[1 1 1] Wait before crossing
      (if (>= (Variables|Default|GetcountdownBeforeCrossing) 0.0)
        (Variables|Default|SetcountdownBeforeCrossing (- (Variables|Default|GetcountdownBeforeCrossing) DeltaSeconds))
        (else
          (Variables|Default|SetAiState "NewEnumerator0")
          (Variables|Default|SetcountdownBeforeCrossing 0.0))))
    (:NewEnumerator0
      (if (not (Variables|Default|GetisCarriedByPlayer))
        ;[1 1 1] Cross the road alone
        (Transformation|AddRelativeLocation "-3.000000, 0, 0" false)
        (if (Math|Vector|Equal(Vector) (Transformation|GetActorLocation) (Variables|Default|GetfinalDestination) 5.0)
          (Variables|Default|SetAiState "NewEnumerator3"))))
    (:NewEnumerator3
      ;[1 1 1] Destruction after 2.0 seconds
      (if (>= (Variables|Default|GetcountdownBeforeDestroy) 0.0)
        (Variables|Default|SetcountdownBeforeDestroy (- (Variables|Default|GetcountdownBeforeDestroy) DeltaSeconds))
        (else
          (Actor|DestroyActor))))))

(fn ConstructionScript)

(fn GrabGrandma
  (if (not (Utilities|Enum|Equal(Enum) (Variables|Default|GetAiState) "NewEnumerator3"))
    (Variables|Default|SetAiState "NewEnumerator0")
    (Variables|Default|SetisCarriedByPlayer true)
    (return (not (Utilities|Enum|Equal(Enum) (Variables|Default|GetAiState) "NewEnumerator3")))))

(fn DropGrandma
  (Variables|Default|SetisCarriedByPlayer false))