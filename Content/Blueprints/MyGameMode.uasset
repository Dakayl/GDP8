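; MyGameMode is a game mode that rations a shared pool of tokens, apparently to throttle spawning.
; Tick feeds a random-length Delay between the min and max spawn times, acting as a repeating timer that adds one token up to MaxTokens.
; GetToken consumes a token when any remain, prints a debug string on success and returns whether spawning is allowed.
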(event EventBeginPlay)

(event EventTick
  (params (DeltaSeconds :type Float%20%28single-precision%29))
  (Utilities|FlowControl|Delay (Math|Random|RandomFloatinRange (Variables|Default|GetminSpawnTime) (Variables|Default|GetmaxSpawnTime)))
  (if (< (Variables|Default|GetnbTokens) (Variables|Default|GetmaxTokens))
    (Variables|Default|SetnbTokens (+ (Variables|Default|GetnbTokens) 1.0))))

(fn ConstructionScript)

(fn GetToken
  (bind _output_get (Variables|Default|SetcanSpawn (> (Variables|Default|GetnbTokens) 0.0)))
  (if _output_get
    (Variables|Default|SetnbTokens (- (Variables|Default|GetnbTokens) 1.0))
    (Development|PrintString (Utilities|String|ToString(Boolean) (Variables|Default|GetcanSpawn))))
  (return (Variables|Default|GetcanSpawn)))