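; GrandmaSpawn is a spawner that repeatedly creates Grandma actors set up to cross a road.
; Tick spawns the first immediately, then uses a latent Delay to space later spawns at random intervals.
; Each Grandma receives its start direction, a crossing direction opposite the spawner's Position, and the arrival zone.
; It also gets a crosswalk point at a random X offset and a final destination one road width away along Z.
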(event EventBeginPlay)

(event EventActorBeginOverlap
  (params (OtherActor :type Actor%20Object%20Reference)))

(event EventTick
  (params (DeltaSeconds :type Float%20%28single-precision%29))
  (bind _returnvalue (Transformation|GetActorLocation))
  (bind (_x _y _z) (Math|Vector|BreakVector _returnvalue))
  (if (Variables|Default|GetfirstSpawn)
    (Variables|Default|SetfirstSpawn false)
    (else
      (Utilities|FlowControl|Delay (Math|Random|RandomFloatinRange (Variables|Default|GetdelayMin) (Variables|Default|GetdelayMax)))))
  (bind _returnvalue_2 (Game|SpawnActorfromClass "/Game/Blueprints/Grandma.Grandma_C" (Math|Transform|MakeTransform _returnvalue (Class|KismetMathLibrary|MakeRot 0.0 (select (Utilities|Enum|Equal(Enum) "NewEnumerator2" (Variables|Default|GetstartDirection)) 0.0 1.8e+02) 0.0)) false 0))
  (bind _output_get (Variables|/Game/Blueprints/Grandma.Grandma_C|SetstartDirection _returnvalue_2 (Variables|Default|GetstartDirection)))
  (Variables|/Game/Blueprints/Grandma.Grandma_C|SetcrossDirection _returnvalue_2 (Utilities|Select :Index (Variables|Default|Getposition) :NewEnumerator0 "NewEnumerator1" :NewEnumerator1 "NewEnumerator0" :NewEnumerator2 "NewEnumerator3" :NewEnumerator3 "NewEnumerator2"))
  (Variables|/Game/Blueprints/Grandma.Grandma_C|Setdirection _returnvalue_2 _output_get)
  (bind _output_get_2 (Variables|/Game/Blueprints/Grandma.Grandma_C|SetcrosswalkPosition _returnvalue_2 (Math|Vector|MakeVector (+ _x (* (Math|Random|RandomFloatinRange (Variables|Default|GetminCrossDistance) (Variables|Default|GetmaxCrossDistance)) (select (Utilities|Enum|Equal(Enum) (Variables|Default|GetstartDirection) "NewEnumerator2") -1.0 1.0))) _y _z)))
  (Variables|/Game/Blueprints/Grandma.Grandma_C|SetfinalDestination _returnvalue_2 (Math|Vector|MakeVector (.X (Math|Vector|BreakVector _output_get_2)) (.Y (Math|Vector|BreakVector _output_get_2)) (+ (.Z (Math|Vector|BreakVector _output_get_2)) (* (Variables|Default|GetroadSize) (select (Utilities|Enum|Equal(Enum) (Variables|Default|Getposition) "NewEnumerator0") -1.0 1.0)))))
  (Variables|/Game/Blueprints/Grandma.Grandma_C|SetarrivalZone _returnvalue_2 (Variables|Default|GetarrivalZone)))

(fn ConstructionScript)